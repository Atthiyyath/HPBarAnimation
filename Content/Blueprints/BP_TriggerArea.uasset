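; BP_TriggerArea is a trigger volume actor that applies damage to the player's health bar when the player enters it.
; Its Sphere overlap checks that the overlapping actor is player 0's BP_ThirdPersonCharacter.
; It then passes its Damage value straight to UpdateHealth on the WBP_HPbar inside the character's HPWidgetComponent and prints that value for debugging.
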(event `self.Sphere.OnComponentBeginOverlap`
  (params (OverlappedComponent :type "PrimitiveComponent Object Reference") (OtherActor :type "Actor Object Reference") (OtherComp :type "PrimitiveComponent Object Reference") (OtherBodyIndex :type Integer) (bFromSweep :type Boolean) (SweepResult :type "HitResult Structure (by ref)"))
  (bind _damage (`self.Damage`))
  (bind _asbp_third_person_character (cast `/Game/ThirdPerson/Blueprints/BP_ThirdPersonCharacter` (`GameplayStatics.GetPlayerCharacter` 0)))
  (if (== _asbp_third_person_character OtherActor)
    (bind _aswbp_hpbar (cast `/Game/Widgets/WBP_HPbar` (`WidgetComponent.GetWidget` (`/Game/ThirdPerson/Blueprints/BP_ThirdPersonCharacter.HPWidgetComponent` _asbp_third_person_character))))
    (`/Engine/EditorBlueprintResources/StandardMacros.IsValid` _aswbp_hpbar
      (:`Is Valid`
        (`HPWidget.UpdateHealth` _aswbp_hpbar _damage)
        (`KismetSystemLibrary.PrintString` (`KismetStringLibrary.Conv_DoubleToString` _damage))))))

(fn `UserConstructionScript`)